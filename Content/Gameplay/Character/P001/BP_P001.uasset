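; Player character Blueprint for P001, handling movement, look, jump, crouch toggle and spring-arm camera zoom and offset through Enhanced Input.
; Move input, doubled while running, is stored as forward, sideways and normalized values and applied relative to control rotation.
; Pressing Run with sideways input plays a left or right dodge montage, guarded by IsDodge.
; Root motion extraction is disabled on jump and restored to montages-only on landing; Tick prints debug input.
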(event Input|EnhancedActionEvents|EnhancedInputActionIA_Move
  (params (ActionValue :type Vector%202D%20Structure) (ElapsedSeconds :type Float%20%28double-precision%29) (TriggeredSeconds :type Float%20%28double-precision%29) (InputAction :type Input%20Action%20Object%20Reference :default "/Game/Gameplay/Input/IA_Move.IA_Move"))
  (bind _returnvalue (Pawn|GetControlRotation :!class /Script/Engine.Pawn))
  (bind _isrunning (Variables|Move|GetIsRunning))
  (bind _returnvalue_2 (Math|Float|SelectFloat 2.0 1.0 _isrunning))
  ;[1 1 1 0.5 30] IA_MOVE
  (:Triggered
    (Utilities|FlowControl|Sequence
      (:then_0
        (Variables|Move|SetForwardInput (* (.y ActionValue) _returnvalue_2))
        (Variables|Move|SetSidewayInput (* (.x ActionValue) _returnvalue_2))
        (Variables|Default|SetNormalizeInputVector (Math|Vector2D|Normalize2D (Math|Vector2D|MakeVector2D (Variables|Move|GetSidewayInput) (Variables|Move|GetForwardInput)))))
      (:then_1
        (Pawn|Input|AddMovementInput (Math|Vector|GetForwardVector _returnvalue) (Variables|Move|GetForwardInput) false)
        (Pawn|Input|AddMovementInput (Math|Vector|GetRightVector _returnvalue) (Variables|Move|GetSidewayInput) false))))
  (:Completed
    (Variables|Move|SetForwardInput 0.0)
    (Variables|Move|SetSidewayInput 0.0)
    (Variables|Default|SetNormalizeInputVector "")))

(event Input|EnhancedActionEvents|EnhancedInputActionIA_Run
  (params (ActionValue :type Boolean) (ElapsedSeconds :type Float%20%28double-precision%29) (TriggeredSeconds :type Float%20%28double-precision%29) (InputAction :type Input%20Action%20Object%20Reference :default "/Game/Gameplay/Input/IA_Run.IA_Run"))
  (bind _mesh (Variables|Character|GetMesh))
  ;[0.15 0.15 0.15 0.5] IA_Run
  (:Triggered
    (Variables|Move|SetIsRunning ActionValue :!label _label))
  (:Started
    (if (and (not (Variables|Move|GetIsDodge)) (!= (Variables|Move|GetSidewayInput) 0.0))
      (Variables|Move|SetIsDodge true)
      (if (< (Variables|Move|GetSidewayInput) 0.0)
        (Animation|Montage|PlayMontage _mesh "/Game/Art/Character/P001/Animations/Standing_Dodge_Left_Montage.Standing_Dodge_Left_Montage"
          (:OnCompleted
            _)
          (:OnBlendOut
            _)
          (:OnInterrupted
            _))
        (else
          (Animation|Montage|PlayMontage _mesh "/Game/Art/Character/P001/Animations/Standing_Dodge_Right_Montage.Standing_Dodge_Right_Montage"
            (:OnCompleted
              _)
            (:OnBlendOut
              _)
            (:OnInterrupted
              _))))
      (Variables|Move|SetIsDodge false)))
  (:Completed
    (goto _label)))

(event Input|EnhancedActionEvents|EnhancedInputActionIA_Look
  (params (ActionValue :type Vector%202D%20Structure) (ElapsedSeconds :type Float%20%28double-precision%29) (TriggeredSeconds :type Float%20%28double-precision%29) (InputAction :type Input%20Action%20Object%20Reference :default "/Game/Gameplay/Input/IA_Look.IA_Look"))
  ;[0.15 0.15 0.15 0.5] IA_Look
  (Pawn|Input|AddControllerYawInput (.x ActionValue))
  (Pawn|Input|AddControllerPitchInput (* (.y ActionValue) -1.0)))

(event Input|EnhancedActionEvents|EnhancedInputActionIA_CameraLength
  (params (ActionValue :type Float%20%28double-precision%29) (ElapsedSeconds :type Float%20%28double-precision%29) (TriggeredSeconds :type Float%20%28double-precision%29) (InputAction :type Input%20Action%20Object%20Reference :default "/Game/Gameplay/Input/IA_CameraLength.IA_CameraLength"))
  (bind _springarm (Variables|Default|GetSpringArm))
  ;[0.15 0.15 0.15 0.5] IA_CameraLength
  (Variables|/Script/Engine.SpringArmComponent|SetTargetArmLength _springarm (Math|Float|Clamp(Float) (+ (* ActionValue 5e+01) (Variables|/Script/Engine.SpringArmComponent|GetTargetArmLength _springarm)) 1e+02 8e+02)))

(event Input|EnhancedActionEvents|EnhancedInputActionIA_CameraPosition
  (params (ActionValue :type Vector%202D%20Structure) (ElapsedSeconds :type Float%20%28double-precision%29) (TriggeredSeconds :type Float%20%28double-precision%29) (InputAction :type Input%20Action%20Object%20Reference :default "/Game/Gameplay/Input/IA_CameraPosition.IA_CameraPosition"))
  (bind _springarm (Variables|Default|GetSpringArm))
  ;[0.15 0.15 0.15 0.5] IA_CameraOffset
  (Variables|/Script/Engine.SpringArmComponent|SetSocketOffset _springarm (Math|Vector|MakeVector (.x (Variables|/Script/Engine.SpringArmComponent|GetSocketOffset _springarm)) (+ (.x ActionValue) (.y (Variables|/Script/Engine.SpringArmComponent|GetSocketOffset _springarm))) (+ (.y ActionValue) (.z (Variables|/Script/Engine.SpringArmComponent|GetSocketOffset _springarm))))))

(event Input|EnhancedActionEvents|EnhancedInputActionIA_Jump
  (params (ActionValue :type Boolean) (ElapsedSeconds :type Float%20%28double-precision%29) (TriggeredSeconds :type Float%20%28double-precision%29) (InputAction :type Input%20Action%20Object%20Reference :default "/Game/Gameplay/Input/IA_Jump.IA_Jump"))
  ;[0.7448 0.7448 0.7448 0.5] IA_JUMP
  (Character|Jump))

(event Input|EnhancedActionEvents|EnhancedInputActionIA_Crouch
  (params (ActionValue :type Boolean) (ElapsedSeconds :type Float%20%28double-precision%29) (TriggeredSeconds :type Float%20%28double-precision%29) (InputAction :type Input%20Action%20Object%20Reference :default "/Game/Gameplay/Input/IA_Crouch.IA_Crouch"))
  ;[0.15 0.15 0.15 0.5 50] IA_Crouch
  (:Started
    (if (Variables|Default|GetbIsCrouched)
      (Character|UnCrouch)
      (else
        (Character|Crouch)))))

(event EventBeginPlay
  (bind _asplayer_controller (Utilities|Casting|CastToPlayerController (Pawn|GetController)))
  (Utilities|IsValid _asplayer_controller
    (:Is%20Valid
      (Input|AddMappingContext (PlayerController|LocalPlayerSubsystems|GetEnhancedInputLocalPlayerSubsystem _asplayer_controller) "/Game/Gameplay/Input/IMC_PlayerHumanControl.IMC_PlayerHumanControl" 0 "(bIgnoreAllPressedKeysUntilRelease=True,bForceImmediately=False,bNotifyUserSettings=False)"))))

(event EventOnJumped
  ;[0.7448 0.7448 0.7448 0.5] IA_JUMP
  (Class|AnimInstance|SetRootMotionMode (Components|SkeletalMesh|GetAnimInstance (Variables|Character|GetMesh)) "NoRootMotionExtraction"))

(event EventOnLanded
  (params (Hit :type Hit%20Result%20Structure%20%28by%20ref%29))
  ;[0.7448 0.7448 0.7448 0.5] IA_JUMP
  (Class|AnimInstance|SetRootMotionMode (Components|SkeletalMesh|GetAnimInstance (Variables|Character|GetMesh)) "RootMotionFromMontagesOnly"))

(event EventTick
  (params (DeltaSeconds :type Float%20%28single-precision%29))
  ;[0.15 0.15 0.15 0.5] Test Input
  (Development|PrintString (Utilities|String|Append "ForwardInput: " (Utilities|String|ToString(Float) (Variables|Move|GetForwardInput)) ", SidewayInput: " (Utilities|String|ToString(Float) (Variables|Move|GetSidewayInput)) ", NormalInputVec:" (Utilities|String|ToString(Vector2d) (Variables|Default|GetNormalizeInputVector))) true true "(R=0.000000,G=0.660000,B=1.000000,A=1.000000)" 0.0))

(fn ConstructionScript)